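; Scene component that emits a toggleable laser, bouncing off "reflection"-tagged components and continuing through "passthrough" ones.
; While active, Tick recursively line-traces the path, with capped bounces, into segments drawn by a resized pool of Niagara systems.
; SendMessages compares hit actors by index against last frame's, firing hit and lost-hit dispatchers and messages to those actors.
; New hits optionally take damage and can start a repeating hit timer.
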(event `self.ReceiveBeginPlay`
  (`self.SetActivate` (`self.bAutoActive`))
  (if (> (`self.MaxBounces`) 57)
    (set `self.MaxBounces` 57)))

(event `self.ReceiveTick`
  (params (DeltaSeconds :type "Float (single-precision)"))
  (if (<= (`self.SetHitTickInterval`) 0.0)
    (set `self.SetHitTickInterval` DeltaSeconds))
  (if (`self.bIsActivate`)
    (`KismetArrayLibrary.Array_Clear` (`self.LasersInfos`))
    (set `self.currentBounce` 0)
    (`self.Set Trace` (`self.K2_GetComponentLocation`) (`self.GetForwardVector`) 1.0)
    (for (_array_element _array_index) (`self.LasersInfos`)
      (if (not (`KismetArrayLibrary.Array_IsValidIndex` (`self.NiagaraSystems`) _array_index))
        (`self.SpawnNiagaraLaser` _array_index))
      (`self.SetNiagaraParameters` (`|GetArrayItem` (`self.NiagaraSystems`) _array_index) _array_element))
    (`self.RemoveNiagaras`)
    (`self.SendMessages`)
    (else
      (set `self.currentBounce` 0)
      (`KismetArrayLibrary.Array_Clear` (`self.LasersInfos`))
      (`self.RemoveNiagaras`)
      (`self.SendMessages`)
      (`KismetSystemLibrary.K2_ClearAndInvalidateTimerHandle` (`self.HitTickIntervalTimerHandle`)))))

(event `S_Enable`
  (params (Enable :type Boolean))
  ;[1 1 1] Replicate laser activation
  (set `self.bIsActivate` Enable))

(fn `ApplyDamage`
  (params (BaseDamage :type "Float (single-precision)"))
  (if (`self.ShouldApplyDamage`)
    (`GameplayStatics.ApplyDamage` (`self.CurrentHitActor`) BaseDamage null null "/Game/AdvancedLaserSystem/Blueprints/BP_Laser_DamageType.BP_Laser_DamageType_C"))
  (return))

(fn `CountNumberLaserBounces`
  (params (Start :type "Vector Structure") (Direction :type "Vector Structure") (RemainDistance :type "Float (double-precision)") (Actor :type "Actor Object Reference"))
  (bind _result (`/Engine/EditorBlueprintResources/StandardMacros.IncrementInt` (`self.currentBounce`))
    (:`  `
      (if (<= _result (`self.MaxBounces`))
        (`self.Set Trace` Start Direction RemainDistance Actor))
      (return))))

(fn `Enable`
  (params (Active :type Boolean))
  (`self.S_Enable` Active)
  (return))

(fn `EnableAndSetActorsToIgnore`
  (params (Active :type Boolean) (`Actors to Ignore` :type "Array of Actor Object Reference (by ref)"))
  (`self.SetActorsToIgnore` `Actors to Ignore`)
  (set `self.bIsActivate` Active)
  (return))

(fn `Get Current Hit`
  (returns (CurrentsHit :type "Array of Actor Object Reference"))
  (return (`self.CurrentHitsActors`)))

(fn `GetLastHitActor`
  (returns (LastHit :type "Array of Actor Object Reference"))
  (return (`self.LastHitsActors`)))

(fn `OnLaserHitMessage`
  (params (Target :type "Object Object Reference") (Index :type Integer))
  (bind _currenthits (`self.CurrentHits`))
  (bind _output (`|GetArrayItem` _currenthits Index))
  (if (> (`KismetArrayLibrary.Array_Length` _currenthits) 0)
    (`self.OnRetrievedLaserHit` _output Index)
    (message `/Game/AdvancedLaserSystem/Blueprints/BPI_LasersCommunication.ReceivedLaserHit` Target _output (`self.GetOwner`) self (`self.LaserName`))
    (return)))

(fn `OnLaserHitMessageOnTick`
  (bind _lasthits (`self.LastHits`))
  (`self.ApplyDamage` (`self.DamageToApply`))
  (for (_array_element _array_index) (`self.LastHitsActors`)
    (if (> (`KismetArrayLibrary.Array_Length` _lasthits) 0)
      (bind _output (`|GetArrayItem` _lasthits _array_index))
      (`self.OnRetrievedLaserHit` _output)
      (message `/Game/AdvancedLaserSystem/Blueprints/BPI_LasersCommunication.ReceivedLaserHit` _array_element _output (`self.GetOwner`) self (`self.LaserName`))))
  (return))

(fn `RemoveNiagaras`
  (bind _niagarasystems (`self.NiagaraSystems`))
  (bind _returnvalue (`KismetArrayLibrary.Array_LastIndex` _niagarasystems))
  (while (> (`KismetArrayLibrary.Array_Length` (`self.NiagaraSystems`)) (`KismetArrayLibrary.Array_Length` (`self.LasersInfos`)))
    (`self.K2_DestroyComponent` (`|GetArrayItem` _niagarasystems _returnvalue))
    (`KismetArrayLibrary.Array_Remove` (`self.NiagaraSystems`) _returnvalue)
    (return))
  (return))

(fn `SendMessages`
  (bind _currenthitsactors (`self.CurrentHitsActors`))
  (bind _currenthits (`self.CurrentHits`))
  ;[0 0.1195 1] If the actors hit on the last frame are different from the current frame, we trigger the event "OnLaserLostHit" and send message "LostReceived".
  (for (_array_element _array_index) (`self.LastHitsActors`)
    (if (`KismetArrayLibrary.Array_IsValidIndex` (`self.CurrentHitsActors`) _array_index)
      (if (not (== (`|GetArrayItem` (`self.CurrentHitsActors`) _array_index) _array_element))
        (bind _output (`|GetArrayItem` (`self.LastHits`) _array_index))
        (`self.OnLostLaserHit` _output _array_index :!label _label)
        (message `/Game/AdvancedLaserSystem/Blueprints/BPI_LasersCommunication.LostLaserHit` _array_element _output (`self.GetOwner`) self (`self.LaserName`)))
      (else
        (goto _label))))
  ;[0 0.1195 1] If the actors hit on the current frame does not exist in last actors hit, we trigger the event "OnLaserHit" and send message "Received".
  (for (_array_element_2 _array_index_2) (`self.CurrentHitsActors`)
    (set `self.CurrentHitActor` _array_element_2)
    (if (`KismetArrayLibrary.Array_IsValidIndex` (`self.LastHitsActors`) _array_index_2)
      (if (not (== (`|GetArrayItem` (`self.LastHitsActors`) _array_index_2) _array_element_2))
        (`self.OnLaserHitMessage` _array_element_2 _array_index_2 :!label _label_2)
        (`self.ApplyDamage` (`self.DamageToApply`))
        (if (`self.LaserHitOnTick`)
          (bind _returnvalue (`KismetSystemLibrary.K2_SetTimerDelegate` (`|CreateDelegate` :!event `OnLaserHitMessageOnTick`) (`self.SetHitTickInterval`) true))
          (set `self.HitTickIntervalTimerHandle` _returnvalue)
          (else
            (`KismetSystemLibrary.K2_ClearAndInvalidateTimerHandle` (`self.HitTickIntervalTimerHandle`)))))
      (else
        (goto _label_2))))
  (set `self.LastHitsActors` _currenthitsactors)
  (`KismetArrayLibrary.Array_Clear` _currenthitsactors)
  (set `self.LastHits` _currenthits)
  (`KismetArrayLibrary.Array_Clear` _currenthits)
  (return))

(fn `Set Trace`
  (params (Start :type "Vector Structure") (Direction :type "Vector Structure") (RemainDistance :type "Float (double-precision)") (Actor :type "Actor Object Reference"))
  (locals (L_RemainDistance :type "Float (double-precision)") (L_Start :type "Vector Structure" :default (0.0 0.0 0.0)) (L_Direction :type "Vector Structure" :default (0.0 0.0 0.0)) (L_Actor :type "Actor Object Reference") (L_Normal :type "Vector Structure" :default (0.0 0.0 0.0)) (L_HitIndex :type Integer))
  ;[0 0.1195 1] Define the end and start location of the laser
  (set `local.L_Start` Start)
  (set `local.L_Direction` Direction)
  (set `self.Remain Distance` RemainDistance)
  (`KismetArrayLibrary.Array_Add` (`self.Actors to Ignore`) Actor)
  (bind (_outhit _returnvalue) (`KismetSystemLibrary.LineTraceSingle` (`local.L_Start`) (+ (`local.L_Start`) (* (`local.L_Direction`) (`self.BeamMaxDistance`))) (`self.Trace Channel`) false (`self.Actors to Ignore`) "None" true (struct :`R` 1.0 :`A` 1.0) (struct :`G` 1.0 :`A` 1.0) 0.0))
  ;[0 0.1195 1] Remove the last actor hit from the actorsToIgnore list
  (`KismetArrayLibrary.Array_RemoveItem` (`self.Actors to Ignore`) Actor)
  (`self.IfLaserHasHitReflectObject` _outhit _returnvalue
    (:`True`
      (bind (_bblockinghit _binitialoverlap _time _distance _location _impactpoint _normal _impactnormal _physmat _hitactor _hitcomponent _hitbonename _bonename _hititem _elementindex _faceindex _tracestart _traceend) (`GameplayStatics.BreakHitResult` _outhit))
      (`KismetArrayLibrary.Array_Add` (`self.CurrentHitsActors`) _hitactor)
      (`KismetArrayLibrary.Array_Add` (`self.CurrentHits`) _outhit)
      (set `local.L_Normal` _normal)
      (set `local.L_RemainDistance` (/ _distance (`self.BeamMaxDistance`)))
      (set `local.L_Start` _location)
      ;[0 0.1195 1] Set the end point of the laser based on whether it should reflect or pass through the surface.
      (set `local.L_Actor` _hitactor)
      (if (`self.ComponentHasTag` _hitcomponent "reflection")
        (set `local.L_Direction` (`KismetMathLibrary.MirrorVectorByNormal` (`local.L_Direction`) (`local.L_Normal`)))
        (`self.CountNumberLaserBounces` (`local.L_Start`) (`local.L_Direction`) (`local.L_RemainDistance`) (`local.L_Actor`))
        (return)
        (else
          (if (`self.ComponentHasTag` _hitcomponent "passthrough")
            (set `local.L_Direction` (`KismetMathLibrary.GetForwardVector` (`KismetMathLibrary.FindLookAtRotation` _tracestart _traceend)))
            (`self.Set Trace` (`local.L_Start`) (`local.L_Direction`) (`local.L_RemainDistance`) (`local.L_Actor`)))
          (return))))
    (:`False`
      (return))))

(fn `SetActivate`
  (params (bIsActivate :type Boolean))
  (set `self.bIsActivate` bIsActivate)
  (return))

(fn `SetActorsToIgnore`
  (params (`Actors to Ignore` :type "Array of Actor Object Reference"))
  (set `self.Actors to Ignore` `Actors to Ignore`)
  (return))

(fn `SetLaserName`
  (params (LaserName :type Name))
  (set `self.LaserName` LaserName)
  (return))

(fn `SetNiagaraParameters`
  (params (NiagaraSystem :type "NiagaraComponent Object Reference") (LaserInfos :type "/Game/AdvancedLaserSystem/Blueprints/S_LasersInfos Structure"))
  (locals (showImpact :type Boolean))
  (`/Engine/EditorBlueprintResources/StandardMacros.IsValid` NiagaraSystem
    (:`Is Valid`
      ;[1 0 0] Required
      ;;[0 0.1195 1] Set the start and the end of the niagara ribbon laser
      (`NiagaraComponent.SetVariableVec3` NiagaraSystem (`self.LaserStart`) LaserInfos_Start_2_6D41E59042DF47E5BBA58D8BD7D92F7B)
      (`NiagaraComponent.SetVariableVec3` NiagaraSystem (`self.LaserEnd`) LaserInfos_End_8_A13E57BC4C77C12941476287EC5B51CE)
      ;[1 0.2635 0] Optionnal but recommanded
      ;;[0 0.1195 1] Control the width of the laser
      (`NiagaraComponent.SetVariableFloat` NiagaraSystem (`self.LaserWidth`) LaserInfos_Width_11_439F11CF40D6F5CA253A66A4E03882ED)
      ;;[0 0.1195 1] These parameters are used to fade the laser at the end
      (`NiagaraComponent.SetVariableFloat` NiagaraSystem (`self.LaserPowerStart`) LaserInfos_PowerStart_14_041C2132407BF735ADCAB19586557DBD)
      (`NiagaraComponent.SetVariableFloat` NiagaraSystem (`self.LaserPowerEnd`) LaserInfos_PowerEnd_15_0C65CA0548AC359D4DDDB4AE316EE6C6)
      ;;[0 0.1195 1] These parameters are used to set a Niagara effect upon the impact of the laser if it is reflected or blocked.
      (if LaserInfos_bIsHit_31_D5638CA2424A8AA5F2AC2CADB949409C
        (set `local.showImpact` (not (`self.ComponentHasTag` (`.HitComponent` (`GameplayStatics.BreakHitResult` LaserInfos_hit_29_63D61E1744E74B68139AC4A1E86265F3)) "through")))
        (`NiagaraComponent.SetVariableVec3` NiagaraSystem (`self.LaserImpactNormal`) LaserInfos_ImpactNormal_6_04B3DCC94B7C59994860639BDCCC0B04)
        (else
          (set `local.showImpact` false)))
      (`NiagaraComponent.SetVariableBool` NiagaraSystem (`self.LaserShowImpact`) (`local.showImpact`))
      ;;[0 0.1195 1] Set the color of the laser
      (`NiagaraComponent.SetVariableLinearColor` NiagaraSystem (`self.LaserColor`) (`self.Color`))
      (return))))

(fn `SpawnNiagaraLaser`
  (params (Index :type Integer))
  (bind _laserniagarasystem (`self.LaserNiagaraSystem`))
  (if (`self.bIsActivate`)
    (`/Engine/EditorBlueprintResources/StandardMacros.IsValid` _laserniagarasystem
      (:`Is Valid`
        (bind _returnvalue (`NiagaraFunctionLibrary.SpawnSystemAtLocation` _laserniagarasystem (0.0 0.0 0.0) (struct) (1.0 1.0 1.0) false))
        (`/Engine/EditorBlueprintResources/StandardMacros.IsValid` _returnvalue
          (:`Is Valid`
            (`KismetArrayLibrary.Array_Set` (`self.NiagaraSystems`) Index _returnvalue true)
            (`NiagaraComponent.SetTickBehavior` _returnvalue "ForceTickLast")
            (return)))))
    (else
      (`self.RemoveNiagaras`))))